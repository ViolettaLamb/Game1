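; BP_Enemy is a stealth-game enemy that is knocked out when the player's third-person character overlaps its capsule.
; On that overlap it plays a quack sound attached to its mesh, turns on physics simulation for the mesh and activates a Niagara effect.
; After a short delay it tells its Manager to remove an enemy and check, then destroys itself.
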(event OnComponentBeginOverlap(Capsule)
  (params (OverlappedComponent :type Primitive%20Component%20Object%20Reference) (OtherActor :type Actor%20Object%20Reference) (OtherComp :type Primitive%20Component%20Object%20Reference) (OtherBodyIndex :type Integer) (bFromSweep :type Boolean) (SweepResult :type Hit%20Result%20Structure%20%28by%20ref%29))
  (Utilities|Casting|CastToBP_ThirdPersonCharacterCustom OtherActor)
  (Audio|SpawnSoundAttached "/Game/Developer/Sound/GoofyQuack.GoofyQuack" (Variables|Default|GetpolySurface21) "None" "0, 0, 0" "0, 0, 0" "KeepRelativeOffset" false 1.0 1.0 0.0 0 0)
  (Physics|SetSimulatePhysics (Variables|Default|GetpolySurface21) true)
  (Components|Activation|Activate (Variables|Default|GetNiagara) false)
  (Utilities|FlowControl|Delay 1.0)
  (Default|RemoveEnemyandCheck (Variables|Default|GetManager))
  (Actor|DestroyActor))

(fn ConstructionScript)