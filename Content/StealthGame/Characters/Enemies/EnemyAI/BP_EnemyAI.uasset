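; Stealth-game enemy AI character that patrols and chases the player on sight.
; Tick chooses between chasing at run speed and walking either through looping target points or to random reachable points.
; PawnSensing sets visibility, which a retriggerable delay clears one second after the last sighting.
; A CanMove flag paces patrol moves with pauses, but chasing overrides it, re-issuing AIMoveTo every tick while the player is visible.
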(event OnSeePawn(PawnSensing)
  (params (Pawn :type Pawn%20Object%20Reference))
  ;[0.15 0.0585 0.1018 0.5] PawnSensing
  (Utilities|FlowControl|Sequence
    (:then_0
      (Utilities|Casting|CastToBP_ThirdPersonCharacterCustom Pawn
        (:then
          (Development|PrintString "Hey! Stop right there!" true true "(R=0.559044,G=0.013308,B=1.000000,A=1.000000)")
          (Variables|Default|SetbPlayerVisible true))
        (:CastFailed
          (Variables|Default|SetbPlayerVisible false))))
    (:then_1
      (Utilities|FlowControl|RetriggerableDelay 1.0)
      (Development|PrintString "Hm.. Must of been the wind." true true "(R=0.519641,G=0.031324,B=1.000000,A=1.000000)")
      (Variables|Default|SetbPlayerVisible false))))

(event Custom|ChasePlayer
  ;[0.0436 0.0419 0.15 0.5] Chase player
  (CallFunction|UpdateWalkSpeed 6e+02)
  (Variables|Default|SetbCanMove false)
  (AI|AIMoveTo self "0, 0, 0" (Game|GetPlayerCharacter 0) 5e+01 false
    (:OnSuccess
      _)
    (:OnFail
      _))
  (Utilities|FlowControl|Delay 3.0)
  (Variables|Default|SetbCanMove true))

(event Custom|PatrolRandom
  ;[0.04148 0.15 0.07672 0.5] Patrol Random
  (CallFunction|UpdateWalkSpeed 2e+02)
  (Variables|Default|SetbCanMove false)
  (AI|AIMoveTo self (.RandomLocation (AI|Navigation|GetRandomReachablePointinRadius (Transformation|GetActorLocation) 2e+03 0 0)) 0 5e+01 false
    (:OnSuccess
      _)
    (:OnFail
      _))
  (Utilities|FlowControl|Delay 3.0)
  (Variables|Default|SetbCanMove true))

(event Custom|MoveToNextPatrolPoint
  ;[0.02838 0.1342 0.15 0.5] Move to partol points
  (CallFunction|UpdateWalkSpeed 2e+02)
  (Variables|Default|SetbCanMove false)
  (AI|AIMoveTo self "0, 0, 0" (Utilities|Array|Get(acopy) (Variables|Default|GetPatrolTargetPoints) (Variables|Default|GetPatrolTargetPointIndex)) 5e+01 false
    (:OnSuccess
      (Utilities|FlowControl|Delay 3.0)
      (Variables|Default|SetbCanMove true)
      (CallFunction|SetNextPatrolPointIndex))
    (:OnFail
      (Utilities|FlowControl|Delay 3.0)
      (Variables|Default|SetbCanMove true))))

(event Custom|SetNextPatrolPointIndex
  ;[0.15 0.08698 0.01 0.5] Set next patrol index with an modulo which is fancy math thing
  (Variables|Default|SetPatrolTargetPointIndex (Math|Integer|%(Integer) (+ (Variables|Default|GetPatrolTargetPointIndex) 1) (Utilities|Array|Length (Variables|Default|GetPatrolTargetPoints)))))

(event EventBeginPlay)

(event Collision|EventActorBeginOverlap
  (params (OtherActor :type Actor%20Object%20Reference)))

(event EventTick
  (params (DeltaSeconds :type Float%20%28single-precision%29))
  (bind _bplayervisible (Variables|Default|GetbPlayerVisible))
  ;[0.0513 0.09021 0.15 0.5] Event Tick for movement of AI
  (if (Variables|Default|GetbCanMove)
    (if _bplayervisible
      (CallFunction|ChasePlayer)
      (elif (Variables|Default|GetbTargetPointMovement)
        (CallFunction|MovetoNextPatrolPoint)
        (else
          (CallFunction|PatrolRandom))))
    (elif _bplayervisible
      (CallFunction|ChasePlayer))))

(fn ConstructionScript)

(fn UpdateWalkSpeed
  (params (NewWalkSpeed :type Float%20%28double-precision%29))
  (Variables|/Script/Engine.CharacterMovementComponent|SetMaxWalkSpeed (Variables|Character|GetCharacterMovement) NewWalkSpeed))