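; Duck enemy AI for a stealth game that patrols, investigates noises, and chases and attacks the player.
; Tick drives AIMoveTo along looping target points or random reachable points, switching to a chase while PawnSensing sees the player.
; A retriggerable delay clears sight after one second without a sighting.
; Attack montage notifies trigger a forward sphere trace that reloads the player's checkpoint on hit, repeating on misses.
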(event OnSeePawn(PawnSensing)
  (params (Pawn :type Pawn%20Object%20Reference))
  ;[0.15 0.0585 0.1018 0.5] PawnSensing
  (Utilities|FlowControl|Sequence
    (:then_0
      (Utilities|Casting|CastToBP_ThirdPersonCharacterCustom Pawn
        (:then
          (Audio|SpawnSoundAttached "/Game/Developer/Sound/RealistcQuack.RealistcQuack" (Variables|Character|GetMesh) "None" "0, 0, 0" "0, 0, 0" "KeepRelativeOffset" false 1.0 1.0 0.0 0 0)
          (Development|PrintString "QUACK! QUACK! QUACK!" true true "(R=0.559044,G=0.013308,B=1.000000,A=1.000000)")
          (Variables|Default|SetbPlayerVisible true))
        (:CastFailed
          (Variables|Default|SetbPlayerVisible false))))
    (:then_1
      (Utilities|FlowControl|RetriggerableDelay 1.0)
      (Audio|SpawnSoundAttached "/Game/Developer/Sound/GoofyQuack.GoofyQuack" (Variables|Character|GetMesh) "None" "0, 0, 0" "0, 0, 0" "KeepRelativeOffset" false 1.0 1.0 0.0 0 0)
      (Development|PrintString "quaackk..? quack quack" true true "(R=0.519641,G=0.031324,B=1.000000,A=1.000000)")
      (Variables|Default|SetbPlayerVisible false))))

(event OnHearNoise(PawnSensing)
  (params (Instigator :type Pawn%20Object%20Reference) (Location :type Vector%20%28by%20ref%29 :default "0, 0, 0") (Volume :type Float%20%28single-precision%29))
  ;[0.15 0.1202 0.02014 0.5] trigger rock sound
  (CallFunction|UpdateWalkSpeed 2e+02)
  (Variables|Default|SetbCanMove false)
  (AI|AIMoveTo self Location Instigator 5e+01 false
    (:OnSuccess
      _)
    (:OnFail
      _))
  (Utilities|FlowControl|Delay 6.0)
  (Variables|Default|SetbCanMove true))

(event Custom|ChasePlayer
  ;[0.0436 0.0419 0.15 0.5] Chase player
  (CallFunction|UpdateWalkSpeed 6e+02)
  (Variables|Default|SetbCanMove false)
  (AI|AIMoveTo self "0, 0, 0" (Game|GetPlayerCharacter 0) 5e+01 false
    (:OnSuccess
      (CallFunction|Attack)
      (Utilities|FlowControl|Delay 3.0)
      (Variables|Default|SetbCanMove true))))

(event Custom|PatrolRandom
  ;[0.04148 0.15 0.07672 0.5] Patrol Random
  (CallFunction|UpdateWalkSpeed 2e+02)
  (Variables|Default|SetbCanMove false)
  (AI|AIMoveTo self (.RandomLocation (AI|Navigation|GetRandomReachablePointinRadius (Transformation|GetActorLocation) 2e+03 0 0)) 0 5e+01 false
    (:OnSuccess
      (Utilities|FlowControl|Delay 3.0)
      (Variables|Default|SetbCanMove true))))

(event Custom|MoveToNextPatrolPoint
  ;[0.02838 0.1342 0.15 0.5] Move to partol points
  (CallFunction|UpdateWalkSpeed 2e+02)
  (Variables|Default|SetbCanMove false)
  (AI|AIMoveTo self "0, 0, 0" (Utilities|Array|Get(acopy) (Variables|Default|GetPatrolTargetPoints) (Variables|Default|GetPatrolTargetPointIndex)) 5e+01 false
    (:OnSuccess
      (Utilities|FlowControl|Delay 3.0)
      (Variables|Default|SetbCanMove true)
      (CallFunction|SetNextPatrolPointIndex))))

(event Custom|SetNextPatrolPointIndex
  ;[0.15 0.08698 0.01 0.5] Set next patrol index with an modulo which is fancy math thing
  (Variables|Default|SetPatrolTargetPointIndex (Math|Integer|%(Integer) (+ (Variables|Default|GetPatrolTargetPointIndex) 1) (Utilities|Array|Length (Variables|Default|GetPatrolTargetPoints)))))

(event Custom|Attack
  (bind _sphere (Variables|Default|GetSphere))
  (bind _returnvalue (Transformation|GetWorldLocation _sphere))
  ;[0.15 0.1407 0.04319 0.5] Bonk
  (Utilities|FlowControl|DoOnce false ; Only Reset Attack on miss.
    (:Completed
      (bind _notifyname (Animation|Montage|PlayMontage (Variables|Character|GetMesh) "/Game/StealthGame/Art/MYMODELS/Ducky/SK_Ducky_Montage.SK_Ducky_Montage") ; Play the AM_Attack_01
        (:OnCompleted
          (if (Variables|Default|GetbHostile) ; Keep attacking if you haven't landed the hit.
            (CallFunction|ResetAttack) ; Resets the Do Once node.
          ))
        (:OnNotifyBegin
          (switch name _notifyname ; Pick the proper attack type(standard when there is more than one type of attack)
            (:AttackDamage
              (Development|PrintString "QUACCCCCCCCCCCCCCCCCCCCCCKKKKKKKK" true true "(R=0.299809,G=0.000000,B=1.000000,A=1.000000)")
              (bind (_outhits _returnvalue_2) (Collision|MultiSphereTraceForObjects _returnvalue (+ _returnvalue (* (Transformation|GetActorForwardVector) (Variables|Default|GetMeleeTraceDistance))) (Variables|Default|GetMeleeTraceRadius) (Utilities|Array|MakeArray "ObjectTypeQuery3") false 0 "None")) ; Trace forward from hand socket.
              (if _returnvalue_2 ; If a pawn is hit in that trace...
                (for _array_element _outhits ; ...loop through the results....
                  (bind _asbp_third_person_character_custom (Utilities|Casting|CastToBP_ThirdPersonCharacterCustom (.HitActor (Collision|BreakHitResult _array_element))))
                  (Default|LoadCheckpoint _asbp_third_person_character_custom)
                  (Variables|Default|SetbHostile false))))))))))

(event Custom|ResetAttack
  (bind _sphere (Variables|Default|GetSphere))
  (bind _returnvalue (Transformation|GetWorldLocation _sphere))
  ;[0.15 0.1407 0.04319 0.5] Bonk
  (Utilities|FlowControl|DoOnce false) ; enters at Reset
)

(event Collision|EventActorBeginOverlap
  (params (OtherActor :type Actor%20Object%20Reference)))

(event EventTick
  (params (DeltaSeconds :type Float%20%28single-precision%29))
  (bind _bplayervisible (Variables|Default|GetbPlayerVisible))
  ;[0.0513 0.09021 0.15 0.5] Event Tick for movement of AI
  (if (Variables|Default|GetbCanMove)
    (if _bplayervisible
      (CallFunction|ChasePlayer)
      (elif (Variables|Default|GetbTargetPointMovement)
        (CallFunction|MovetoNextPatrolPoint)
        (else
          (CallFunction|PatrolRandom))))
    (elif _bplayervisible
      (CallFunction|ChasePlayer))))

(fn ConstructionScript)

(fn UpdateWalkSpeed
  (params (NewWalkSpeed :type Float%20%28double-precision%29))
  (Variables|/Script/Engine.CharacterMovementComponent|SetMaxWalkSpeed (Variables|Character|GetCharacterMovement) NewWalkSpeed))

(fn NewFunction
  (CallFunction|ResetAttack))